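; BP_Blaster is a dual-mode weapon that fires rockets or uses a laser to collect water pickups.
; Every tick a debug-drawn forward line trace caches the hit actor and shows impact sparks while the laser is on.
; Collect attaches a laser emitter and, after a delay, destroys a hit actor whose class name contains PickUpWater.
; Fire spawns velocity-driven rockets on a looping timer, owned and instigated by the parent actor.
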(event EventStartCollect
  ;[1 1 1] Laser
  (Variables|Default|SetIsLaser? true)
  (bind _pslaser (CallFunction|SpawnLaser))
  (Utilities|FlowControl|Delay (Variables|Default|GetDropRate))
  (bind _ps (CallFunction|DestroyPickUp (Variables|Default|GetHitingActor)))
  (Utilities|IsValid _ps
    (:Is%20Valid
      (Utilities|FlowControl|Delay (Variables|Default|GetDropRate))
      (Components|DestroyComponent _ps))))

(event EventStartFire
  ;[1 1 1] Fire
  (Variables|Default|SetIsFiring? true)
  (CallFunction|SpawnRocket)
  (Utilities|Time|SetTimerbyFunctionName 0 "SpawnRocket" (Variables|Default|GetRocketRate) true))

(event EventEndFire
  ;[1 1 1] Fire
  (Variables|Default|SetIsFiring? false)
  (Utilities|Time|ClearTimerbyFunctionName 0 "SpawnRocket"))

(event EventEndCollect
  ;[1 1 1] Laser
  (Utilities|FlowControl|Delay (Variables|Default|GetLaserRate))
  (Variables|Default|SetIsLaser? false)
  (Utilities|IsValid (stale EventStartCollect _pslaser)
    (:Is%20Valid
      (Components|DestroyComponent (stale EventStartCollect _pslaser)))))

(event EventTick
  (params (DeltaSeconds :type Float%20%28single-precision%29))
  (bind _arrow (Variables|Default|GetArrow))
  (bind _returnvalue (Transformation|GetWorldLocation _arrow))
  ;[1 1 1] Trasert
  (bind _outhit (Collision|LineTraceByChannel _returnvalue (+ _returnvalue (* (Math|Vector|GetForwardVector (Transformation|GetWorldRotation _arrow)) 3000)) "TraceTypeQuery1" false 0 "ForOneFrame"))
  (bind _output_get (Variables|Default|SetHitingActor (.hitactor _outhit)))
  (if (Variables|Default|GetIsLaser?)
    (Utilities|IsValid _output_get
      (:Is%20Valid
        (if (>= (.distance _outhit) 0.0)
          (if (<= (.distance _outhit) 3e+03)
            (if (>= (.time _outhit) 0.0)
              (Effects|SpawnEmitteratLocation "/Game/Effects/Impacts/P_Metal_Impact.P_Metal_Impact" (.location _outhit)))))))))

(fn ConstructionScript)

(fn SpawnRocket
  (bind _returnvalue (Actor|GetParentActor))
  (bind _barrelarrow (Variables|Default|GetBarrelArrow))
  (bind _returnvalue_2 (Transformation|GetWorldTransform _barrelarrow))
  (bind (_roll _pitch _yaw) (Math|Rotator|BreakRotator (.rotation _returnvalue_2)))
  (bind _returnvalue_3 (Game|SpawnActorfromClass (Variables|Default|GetRocket%20Class) (Math|Transform|MakeTransform (.location _returnvalue_2) (Math|Rotator|MakeRotator _roll _pitch _yaw) "1,1,1") "AlwaysSpawn" _returnvalue 0 1.0 (.AsPawn (Utilities|Casting|CastToPawn _returnvalue))))
  (Physics|SetPhysicsLinearVelocity (Variables|/Game/Blueprints/Weapons/BP_Rocket.BP_Rocket_C|GetRocket _returnvalue_3) (* (Math|Vector|GetForwardVector _barrelarrow) (Variables|Default|GetRocket%20Velocity)) true "None"))

(fn SpawnLaser
  (bind _barrelarrow (Variables|Default|GetBarrelArrow))
  (if (Variables|Default|GetIsLaser?)
    (bind _returnvalue (Effects|SpawnEmitterAttached "/Game/Blueprints/Weapons/PS_Laser.PS_Laser" _barrelarrow "None" (Transformation|GetWorldLocation _barrelarrow) (Transformation|GetWorldRotation _barrelarrow) "0.500000,0.500000,0.500000" "KeepWorldPosition"))
    (return _returnvalue)))

(fn DestroyPickUp
  (params (Hit%20Actor :type Actor%20Object%20Reference))
  (Utilities|IsValid Hit%20Actor
    (:Is%20Valid
      (if (Utilities|String|Contains (Utilities|GetClassDisplayName (Utilities|GetClass Hit%20Actor)) "PickUpWater")
        (bind _returnvalue (Effects|SpawnEmitteratLocation "/Game/Effects/Sparks/P_WeldSparks_NoFakekeBounce.P_WeldSparks_NoFakekeBounce" (Transformation|GetActorLocation Hit%20Actor)))
        (Actor|DestroyActor Hit%20Actor)
        (return _returnvalue)))))