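; BP_Rocket is a rocket projectile that explodes when its capsule hits something.
; The construction script applies configurable mesh, material, scale and mass, sizing the capsule from the scale.
; Hits play a sound, spawn an explosion and hide the rocket.
; Damageable targets also take damage and impulse, spawn water pickups if their class name matches rock or destructible, and are randomly destroyed after the rocket destroys itself.
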(event OnComponentHit(Capsule)
  (params (HitComponent :type Primitive%20Component%20Object%20Reference) (OtherActor :type Actor%20Object%20Reference) (OtherComp :type Primitive%20Component%20Object%20Reference) (NormalImpulse :type Vector :default "0, 0, 0") (Hit :type Hit%20Result%20Structure%20%28by%20ref%29))
  (bind _returnvalue (Utilities|GetClass OtherActor))
  (bind _returnvalue_2 (Transformation|GetActorTransform))
  (bind _returnvalue_3 (Utilities|GetClassDisplayName _returnvalue))
  (Audio|PlaySound2D "/Game/Sounds/DeathFlash.DeathFlash")
  (if (Variables|/Script/Engine.Actor|GetbCanBeDamaged OtherActor)
    (Utilities|FlowControl|Sequence
      (:then_0
        (Game|Damage|ApplyDamage OtherActor 1e+02 (Game|GetInstigatorController) self "/Engine/EngineDamageTypes/DmgTypeBP_Environmental.DmgTypeBP_Environmental_C")
        (Effects|SpawnEmitteratLocation "/Game/Effects/Explosions/P_DPW_bot_tank_explo.P_DPW_bot_tank_explo" (.location _returnvalue_2) (.rotation _returnvalue_2) "2.000000,2.000000,2.000000" :!label _label)
        (Variables|Default|SetHitLocation (.location _returnvalue_2))
        (Rendering|SetActorHiddenInGame true))
      (:then_1
        (Physics|AddImpulse OtherComp (* NormalImpulse 5e+02) "None" true)
        (if (or (Utilities|String|Contains _returnvalue_3 "rock") (Utilities|String|Contains _returnvalue_3 "destruct"))
          (Utilities|FlowControl|Delay 0.2)
          (Game|SpawnActorfromClass "/Game/Blueprints/Weapons/BP_PickUpWater.BP_PickUpWater_C" (Math|Transform|MakeTransform (Variables|Default|GetHitLocation) "0, 0, 0" "1,1,1") "Undefined" 0 0))
        (Actor|DestroyActor)
        (if (> (Math|Random|RandomIntegerinRange 0 1) 0)
          (Actor|DestroyActor OtherActor))))
    (else
      (goto _label))))

(event EventBeginPlay)

(event Collision|EventActorBeginOverlap
  (params (OtherActor :type Actor%20Object%20Reference)))

(event EventTick
  (params (DeltaSeconds :type Float%20%28single-precision%29)))

(fn ConstructionScript
  (bind _capsule (Variables|Default|GetCapsule))
  (bind _rocketscale (Variables|Default|GetRocketScale))
  (Utilities|FlowControl|Sequence
    (:then_0
      (Components|Capsule|SetCapsuleRadius _capsule (* (Math|Vector|GetMaxElement _rocketscale) (Variables|Default|GetCollisionScale)) false)
      (Class|PrimitiveComponent|SetMassScale _capsule "None" (Variables|Default|GetRocketMassScale)))
    (:then_1
      (Components|StaticMesh|SetStaticMesh (Variables|Default|GetRocket) (Variables|Default|GetRocketMesh))
      (Transformation|SetRelativeScale3D (Variables|Default|GetRocket) _rocketscale)
      (bind _rocketmaterial (Variables|Default|GetRocketMaterial)
        (:then
          (Rendering|Material|SetMaterial (Variables|Default|GetRocket) 0 _rocketmaterial))
        (:else)))))